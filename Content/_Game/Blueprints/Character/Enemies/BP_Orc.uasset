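; BP_Orc is an enemy that hurts the player on capsule overlap, with health and material colors set by its Power tier from its Spawner.
; Non-lethal hits knock it backward and briefly flash random palette colors before restoring its tier materials.
; On death it may drop a random item, raises the HUD combo modifier and Power-scaled score, then has the Spawner destroy it.
; Without a valid Spawner at BeginPlay, it shows an error material.
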(event OnComponentBeginOverlap(CapsuleComponent)
  (params (OverlappedComponent :type Primitive%20Component%20Object%20Reference) (OtherActor :type Actor%20Object%20Reference) (OtherComp :type Primitive%20Component%20Object%20Reference) (OtherBodyIndex :type Integer) (bFromSweep :type Boolean) (SweepResult :type Hit%20Result%20Structure%20%28by%20ref%29))
  (bind _asbp_ratt_character (Utilities|Casting|CastToBP_RattCharacter OtherActor))
  (if (not (Variables|/Game/_Game/Blueprints/Character/Player/BP_RattCharacter.BP_RattCharacter_C|GetbIsHurt _asbp_ratt_character))
    (Default|Hurt _asbp_ratt_character self)))

(event Custom|Hurt
  (bind _power (Variables|Default|GetPower))
  (bind _mesh (Variables|Character|GetMesh))
  (bind _spawner (Variables|Default|GetSpawner))
  (bind _capsulecomponent (Variables|Collision|GetCapsuleComponent))
  (bind _result (Math|Integer|DecrementInt (Variables|Default|GetHealth))
    (:%20%20
      (if (<= _result 0)
        (CallFunction|DropRandomItem)
        (bind _asbp_ratt_character (Utilities|Casting|CastToBP_RattCharacter (Game|GetPlayerCharacter 0)))
        (Variables|/Game/_Game/Blueprints/UI/HUD/WBP_Combo.WBP_Combo_C|SetModifier (Variables|/Game/_Game/Blueprints/UI/HUD/WBP_HUD.WBP_HUD_C|GetWBP_Combo (Variables|/Game/_Game/Blueprints/Character/Player/BP_RattCharacter.BP_RattCharacter_C|GetHUD _asbp_ratt_character)) (+ (Variables|/Game/_Game/Blueprints/UI/HUD/WBP_Combo.WBP_Combo_C|GetModifier (Variables|/Game/_Game/Blueprints/UI/HUD/WBP_HUD.WBP_HUD_C|GetWBP_Combo (Variables|/Game/_Game/Blueprints/Character/Player/BP_RattCharacter.BP_RattCharacter_C|GetHUD _asbp_ratt_character))) 1))
        (Variables|/Game/_Game/Blueprints/UI/HUD/WBP_Combo.WBP_Combo_C|SetBaseScore (Variables|/Game/_Game/Blueprints/UI/HUD/WBP_HUD.WBP_HUD_C|GetWBP_Combo (Variables|/Game/_Game/Blueprints/Character/Player/BP_RattCharacter.BP_RattCharacter_C|GetHUD _asbp_ratt_character)) (+ (Variables|/Game/_Game/Blueprints/UI/HUD/WBP_Combo.WBP_Combo_C|GetBaseScore (Variables|/Game/_Game/Blueprints/UI/HUD/WBP_HUD.WBP_HUD_C|GetWBP_Combo (Variables|/Game/_Game/Blueprints/Character/Player/BP_RattCharacter.BP_RattCharacter_C|GetHUD _asbp_ratt_character))) (* (+ (Variables|Default|GetPower) 1) 100)))
        (Default|DestroyOrc (Variables|Default|GetSpawner) self)
        (else
          (Transformation|SetWorldLocation _capsulecomponent (+ (Transformation|GetWorldLocation _capsulecomponent) (* (Math|Vector|GetForwardVector _capsulecomponent) -50)) false true)
          (CallFunction|HurtAnimation)
          (Utilities|FlowControl|Delay 0.2)
          (Rendering|Material|SetMaterial _mesh 0 (Utilities|Array|Get(acopy) (Variables|/Game/_Game/Blueprints/Character/Enemies/BP_OrcSpawner.BP_OrcSpawner_C|GetPowerColorList0 _spawner) _power))
          (Rendering|Material|SetMaterial _mesh 1 (Utilities|Array|Get(acopy) (Variables|/Game/_Game/Blueprints/Character/Enemies/BP_OrcSpawner.BP_OrcSpawner_C|GetPowerColorList1 _spawner) _power)))))))

(event EventBeginPlay
  (bind _power (Variables|Default|GetPower))
  (bind _mesh (Variables|Character|GetMesh))
  (bind _spawner (Variables|Default|GetSpawner))
  (Utilities|IsValid (Variables|Default|GetSpawner)
    (:Is%20Valid
      (Variables|Default|SetHealth (+ (Variables|Default|GetPower) 1))
      (Rendering|Material|SetMaterial _mesh 0 (Utilities|Array|Get(acopy) (Variables|/Game/_Game/Blueprints/Character/Enemies/BP_OrcSpawner.BP_OrcSpawner_C|GetPowerColorList0 _spawner) _power))
      (Rendering|Material|SetMaterial _mesh 1 (Utilities|Array|Get(acopy) (Variables|/Game/_Game/Blueprints/Character/Enemies/BP_OrcSpawner.BP_OrcSpawner_C|GetPowerColorList1 _spawner) _power)))
    (:Is%20Not%20Valid
      (Rendering|Material|SetMaterial (Variables|Character|GetMesh) 0 "/Engine/EngineDebugMaterials/MaterialError_Mat.MaterialError_Mat")
      (Rendering|Material|SetMaterial (Variables|Character|GetMesh) 1 "/Engine/EngineDebugMaterials/MaterialError_Mat.MaterialError_Mat"))))

(fn ConstructionScript)

(fn HurtAnimation
  (bind _mesh (Variables|Character|GetMesh))
  (bind _spawner (Variables|Default|GetSpawner))
  (bind _powercolorlist1 (Variables|/Game/_Game/Blueprints/Character/Enemies/BP_OrcSpawner.BP_OrcSpawner_C|GetPowerColorList1 _spawner))
  (Utilities|FlowControl|Sequence
    (:then_0
      (bind _output (CallFunction|GetRandomColor _powercolorlist1))
      (Rendering|Material|SetMaterial (Variables|Character|GetMesh) 0 _output))
    (:then_1
      (bind _output_2 (CallFunction|GetRandomColor _powercolorlist1 :!label _label))
      (if (== _output_2 (Utilities|Array|Get(acopy) _powercolorlist1 (Variables|Default|GetPower)))
        (goto _label)
        (elif (== _output_2 (Rendering|Material|GetMaterial _mesh 0))
          (goto _label)
          (else
            (Rendering|Material|SetMaterial _mesh 1 _output_2)))))))

(fn GetRandomColor
  (params (ColorList :type Array%20of%20Material%20Interface%20Object%20References))
  (return (Utilities|Array|Get(acopy) ColorList (Math|Random|RandomInteger (Utilities|Array|Length ColorList)))))

(fn DropRandomItem
  (if (<= (Math|Random|RandomInteger 10) 0)
    (bind _output_get (LocalVariables|SetRandomChosenIndex (Math|Random|RandomInteger 3)))
    (switch int _output_get
      (:0
        _)
      (:1
        _)
      (:2
        (LocalVariables|SetRandomChosenIndex (+ (/ (Math|Random|RandomInteger 5) 2) (LocalVariables|GetRandomChosenIndex)))))
    (Game|SpawnActorfromClass (Utilities|Array|Get(acopy) (Variables|Default|GetDropList) (LocalVariables|GetRandomChosenIndex)) (Math|Transform|MakeTransform (Transformation|GetWorldLocation (Variables|Collision|GetCapsuleComponent)) "0.000000,90.000000,-90.000000" "1.000000,1.000000,1.000000") "AlwaysSpawn" "MultiplyWithRoot" 0 0)
    (return)
    (else
      (return))))
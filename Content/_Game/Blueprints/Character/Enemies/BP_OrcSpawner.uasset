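; BP_OrcSpawner runs endless, timed waves of BP_Orc when activated, growing each wave's count and delay and updating the player's HUD wave number.
; Orcs spawn at random navmesh-reachable points around the world origin, skipping attempts that fail a box check around the player's clamped position.
; Each orc's power comes from cascading rolls against per-power spawn rates.
; DestroyOrc tallies deaths by power, raising that rate every hundred.
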(event Custom|SpawnOrcs
  (bind _returnvalue (Game|Player|GetPlayerPawn 0))
  (bind _returnvalue_2 (Math|Random|RandomUnitVector))
  (bind _minspawnrange (Variables|Default|GetMinSpawnRange))
  (bind _maxspawnrange (Variables|Default|GetMaxSpawnRange))
  (bind _returnvalue_3 (Math|Conversions|ToFloat(Integer) _minspawnrange))
  (bind _returnvalue_4 (Math|Conversions|ToFloat(Integer) _maxspawnrange))
  (bind _returnvalue_5 (Transformation|GetActorLocation _returnvalue))
  (bind _returnvalue_6 (* _returnvalue_2 "1.000000,1.000000,0.000000"))
  (bind _returnvalue_7 (Math|Float|Clamp(Float) (.y _returnvalue_5) -7e+02 7e+02))
  (bind _returnvalue_8 (Math|Float|Clamp(Float) (.x _returnvalue_5) -9e+02 9e+02))
  (bind _returnvalue_9 (Math|Random|RandomFloatinRange _returnvalue_3 _returnvalue_4))
  (bind _returnvalue_10 (Math|Vector|MakeVector _returnvalue_8 _returnvalue_7 0.0))
  (bind _returnvalue_11 (* _returnvalue_6 _returnvalue_9))
  (bind _returnvalue_12 (Math|Float|Clamp(Float) (.x _returnvalue_11) -3.5e+03 3.5e+03))
  (bind _returnvalue_13 (Math|Float|Clamp(Float) (.y _returnvalue_11) -3.5e+03 3.5e+03))
  (bind _returnvalue_14 (Math|Vector|MakeVector _returnvalue_12 _returnvalue_13 0.0))
  (bind _randomlocation (AI|Navigation|GetRandomReachablePointinRadius _returnvalue_14 5e+01 0 0))
  (Math|Integer|IncrementInt (Variables|Default|GetWaveNumber)
    (:%20%20
      (for _index (range 0 (- (Variables|Default|GetOrcNumberWave) 1))
        (if (not (or (Math|Float|InRange(Float) (.x _randomlocation) (- (.x _returnvalue_10) 1e+03) (+ (.x _returnvalue_10) 1e+03)) (Math|Float|InRange(Float) (.y _randomlocation) (- (.y _returnvalue_10) 1e+03) (+ (.y _returnvalue_10) 1e+03))))
          (bind _power (CallFunction|SetRandomPower 20))
          (Game|SpawnActorfromClass "/Game/_Game/Blueprints/Character/Enemies/BP_Orc.BP_Orc_C" (Math|Transform|MakeTransform (Math|Vector|MakeVector (.x _randomlocation) (.y _randomlocation) (.z _randomlocation)) "0, 0, 0" "1.000000,1.000000,1.000000") "AdjustIfPossibleButDontSpawnIfColliding" "MultiplyWithRoot" 0 _power self 0)
          (Math|Integer|IncrementInt (Variables|Default|GetOrcsLeft))))
      (Utilities|FlowControl|Delay (+ (Variables|Default|GetDurationBetweenWaves) (Math|Float|Log (Math|Conversions|ToFloat(Integer) (Variables|Default|GetWaveNumber)) 2.0)))
      (Variables|Default|SetOrcNumberWave (+ (Variables|Default|GetOrcNumberWave) (Variables|Default|GetWaveNumber)))
      (bind _asbp_ratt_character (Utilities|Casting|CastToBP_RattCharacter (Game|GetPlayerCharacter 0)))
      (Variables|/Game/_Game/Blueprints/UI/HUD/WBP_Waves.WBP_Waves_C|SetWave (Variables|/Game/_Game/Blueprints/UI/HUD/WBP_HUD.WBP_HUD_C|GetWBP_Waves (Variables|/Game/_Game/Blueprints/Character/Player/BP_RattCharacter.BP_RattCharacter_C|GetHUD _asbp_ratt_character)) (Variables|Default|GetWaveNumber))
      (CallFunction|SpawnOrcs))))

(event Custom|DestroyOrc
  (params (Orc :type BP%20Orc%20Object%20Reference))
  (Math|Integer|IncrementInt (Utilities|Array|Get(acopy) (Variables|Default|GetPowerScores) (Variables|/Game/_Game/Blueprints/Character/Enemies/BP_Orc.BP_Orc_C|GetPower Orc))
    (:%20%20
      (Actor|DestroyActor Orc)
      (Math|Integer|DecrementInt (Variables|Default|GetOrcsLeft)
        (:%20%20
          (for (_array_element _array_index) (Variables|Default|GetPowerScores)
            (if (>= _array_element 100)
              (Utilities|Array|SetArrayElem (Variables|Default|GetPowerScores) _array_index (- _array_element 100))
              (Math|Integer|IncrementInt (Utilities|Array|Get(acopy) (Variables|Default|GetPowerSpawnRates) _array_index)))))))))

(event EventBeginPlay
  (if (Variables|Default|GetActivate)
    (for _array_element (Variables|Default|GetPowerColorList0)
      (Utilities|Array|Add (Variables|Default|GetPowerScores) 0)
      (Utilities|Array|Add (Variables|Default|GetPowerSpawnRates) 1))
    (CallFunction|SpawnOrcs)))

(fn ConstructionScript)

(fn SetRandomPower
  (params (Exclusive%20Max :type Integer))
  (bind (_array_element _array_index) (Utilities|Array|ForEachLoopwithBreak (Variables|Default|GetPowerSpawnRates) :!label _label)
    (:LoopBody
      (if (not (<= (Math|Random|RandomInteger Exclusive%20Max) _array_element))
        (goto _label Break)))
    (:Completed
      (return _array_index))))
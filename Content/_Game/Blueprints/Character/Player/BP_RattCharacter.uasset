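; BP_RattCharacter is the player character, handling movement, shooting, knife slashes, health, pausing and game over.
; Weapons spawn as attached actors from WeaponList; switching skips slots without ammo and NoAmmoLeft returns to the first weapon.
; Hurt removes health, ends the combo, knocks the player back and briefly applies two differing random materials.
; It creates the HUD, pushes health and ammo to it, and passes wave, score and life to the game-over widget.
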(event Custom|EndGame
  (bind _returnvalue (Game|GetPlayerController 0))
  (bind _hud (Variables|Default|GetHUD))
  (bind _returnvalue_2 (UserInterface|CreateWidget "/Game/_Game/Blueprints/UI/WBP_GameOver.WBP_GameOver_C"))
  (UserInterface|Viewport|AddtoViewport _returnvalue_2 0)
  (Variables|/Script/Engine.PlayerController|SetbShowMouseCursor _returnvalue true)
  (Input|SetInputModeUIOnly _returnvalue _returnvalue_2 "DoNotLock" false)
  (Variables|/Game/_Game/Blueprints/UI/WBP_GameOver.WBP_GameOver_C|SetWaveNuber _returnvalue_2 (Variables|/Game/_Game/Blueprints/UI/HUD/WBP_Waves.WBP_Waves_C|GetWave (Variables|/Game/_Game/Blueprints/UI/HUD/WBP_HUD.WBP_HUD_C|GetWBP_Waves _hud)))
  (Variables|/Game/_Game/Blueprints/UI/WBP_GameOver.WBP_GameOver_C|SetBaseScore _returnvalue_2 (Variables|/Game/_Game/Blueprints/UI/HUD/WBP_Score.WBP_Score_C|GetScore (Variables|/Game/_Game/Blueprints/UI/HUD/WBP_HUD.WBP_HUD_C|GetWBP_Score _hud)))
  (Variables|/Game/_Game/Blueprints/UI/WBP_GameOver.WBP_GameOver_C|SetLifeLeft _returnvalue_2 (Variables|Default|GetHealth))
  (Actor|DestroyActor))

(event Input|EnhancedActionEvents|EnhancedInputActionIA_Pause
  (params (ActionValue :type Boolean) (ElapsedSeconds :type Float%20%28double-precision%29) (TriggeredSeconds :type Float%20%28double-precision%29) (InputAction :type Input%20Action%20Object%20Reference :default "/Game/_Game/Blueprints/Input/IA_Pause.IA_Pause"))
  (bind _returnvalue (Game|GetPlayerController 0))
  (:Started
    (bind _returnvalue_2 (UserInterface|CreateWidget "/Game/_Game/Blueprints/UI/WBP_Pause.WBP_Pause_C"))
    (UserInterface|Viewport|AddtoViewport _returnvalue_2 0)
    (Variables|/Script/Engine.PlayerController|SetbShowMouseCursor _returnvalue true)
    (Input|SetInputModeUIOnly _returnvalue 0 "DoNotLock" false)
    (Game|SetGamePaused true)))

(event EventBeginPlay
  (bind _returnvalue (Game|GetPlayerController 0))
  (bind _returnvalue_2 (Game|GetPlayerController 0))
  (bind _ammolist (Variables|Default|GetAmmoList))
  (Utilities|FlowControl|Sequence
    (:then_0
      (Variables|/Script/Engine.PlayerController|SetbShowMouseCursor _returnvalue_2 false)
      (Input|SetInputModeGameOnly _returnvalue_2 false))
    (:then_1
      (bind _returnvalue_3 (UserInterface|CreateWidget "/Game/_Game/Blueprints/UI/HUD/WBP_HUD.WBP_HUD_C" (Game|GetPlayerController 0)))
      (bind _output_get (Variables|Default|SetHUD _returnvalue_3))
      (UserInterface|Viewport|AddtoViewport _output_get 0)
      (CallFunction|HealthUpdate))
    (:then_2
      (CallFunction|ChangeWeaponMesh)
      (Variables|Default|SetbIsHurt false)
      (for _index (range 0 (- (Utilities|Array|Length (Variables|Default|GetWeaponList)) 1))
        (Utilities|Array|Add _ammolist 0))
      (Utilities|Array|SetArrayElem _ammolist 0 1))
    (:then_3
      (Utilities|FlowControl|Delay 0.2)
      (if (Variables|/Script/Engine.PlayerController|GetbShowMouseCursor _returnvalue)
        (Variables|/Script/Engine.PlayerController|SetbShowMouseCursor _returnvalue false)))))

(event Input|EnhancedActionEvents|EnhancedInputActionIA_RattMovement
  (params (ActionValue :type Vector%202D%20Structure) (ElapsedSeconds :type Float%20%28double-precision%29) (TriggeredSeconds :type Float%20%28double-precision%29) (InputAction :type Input%20Action%20Object%20Reference :default "/Game/_Game/Blueprints/Input/IA_RattMovement.IA_RattMovement"))
  (bind _returnvalue (Pawn|GetControlRotation :!class /Script/Engine.Pawn))
  (bind _returnvalue_2 (Math|Rotator|MakeRotator 0.0 0.0 (.yaw _returnvalue)))
  (Utilities|FlowControl|Sequence
    (:then_0
      (Pawn|Input|AddMovementInput (Math|Vector|GetRightVector _returnvalue_2) (.x ActionValue) false))
    (:then_1
      (Pawn|Input|AddMovementInput (Math|Vector|GetForwardVector _returnvalue_2) (.y ActionValue) false))))

(event EventLookat
  (params (Target :type Vector :default "0, 0, 0"))
  (bind _returnvalue (Transformation|GetActorLocation))
  (Transformation|SetActorRotation (Math|Rotator|FindLookatRotation (Math|Vector|MakeVector (.x _returnvalue) (.y _returnvalue) 0.0) (Math|Vector|MakeVector (.x Target) (.y Target) 0.0))))

(event Custom|Hurt
  (params (Attacker :type Actor%20Object%20Reference))
  (bind _mesh (Variables|Character|GetMesh))
  (bind _capsulecomponent (Variables|Collision|GetCapsuleComponent))
  (Variables|Default|SetbIsHurt true)
  (bind _result (Math|Integer|DecrementInt (Variables|Default|GetHealth))
    (:%20%20
      (CallFunction|HealthUpdate)
      (Default|EndCombo (Variables|/Game/_Game/Blueprints/UI/HUD/WBP_HUD.WBP_HUD_C|GetWBP_Combo (Variables|Default|GetHUD)))
      (if (<= _result 0)
        (CallFunction|EndGame)
        (else
          (Transformation|SetWorldLocation _capsulecomponent (+ (Transformation|GetWorldLocation _capsulecomponent) (* (Math|Vector|GetForwardVector (Variables|/Script/Engine.Actor|GetRootComponent Attacker)) 100)) false true)
          (Utilities|FlowControl|Sequence
            (:then_0
              (bind _output (CallFunction|GetRandomColor (Variables|Default|GetHurtColorList)))
              (Rendering|Material|SetMaterial (Variables|Character|GetMesh) 0 _output))
            (:then_1
              (bind _output_2 (CallFunction|GetRandomColor (Variables|Default|GetHurtColorList) :!label _label))
              (if (== _output_2 (Rendering|Material|GetMaterial _mesh 0))
                (goto _label)
                (else
                  (Rendering|Material|SetMaterial _mesh 1 _output_2))))
            (:then_2
              (Utilities|FlowControl|Delay (Variables|Default|GetHurtDuration))
              (Rendering|Material|SetMaterial (Variables|Character|GetMesh) 0 "/Game/Characters/Mannequins/Materials/Manny/MI_Manny_01_New.MI_Manny_01_New")
              (Rendering|Material|SetMaterial (Variables|Character|GetMesh) 1 "/Game/Characters/Mannequins/Materials/Manny/MI_Manny_02_New.MI_Manny_02_New")
              (Variables|Default|SetbIsHurt false))))))))

(event Custom|NoAmmoLeft
  ;[1 0 0 0.5] WeaponSystem
  (bind _output_get (Variables|Default|SetWeaponIndex 0))
  (Utilities|IsValid (Variables|Default|GetCurrentWeaponActor)
    (:Is%20Valid
      (Actor|DestroyActor (Variables|Default|GetCurrentWeaponActor)))
    (:Is%20Not%20Valid
      _))
  (bind _returnvalue (Game|SpawnActorfromClass (Utilities|Array|Get(acopy) (Variables|Default|GetWeaponList) _output_get) (Math|Transform|MakeTransform "0, 0, 0" "0, 0, 0" "0.000000,0.000000,0.000000") "AlwaysSpawn" "MultiplyWithRoot" 0 0))
  (bind _output_get_2 (Variables|Default|SetCurrentWeaponActor _returnvalue))
  (Transformation|AttachComponentToComponent _output_get_2 (Variables|Collision|GetCapsuleComponent) "" "SnapToTarget" "SnapToTarget" "SnapToTarget" true)
  (Transformation|SetActorRelativeTransform _output_get_2 (Math|Transform|MakeTransform "20.000000,15.000000,60.000000" "0, 0, 0" "0.250000,0.250000,0.250000") false false))

(event Custom|ChangeWeaponMesh
  ;[1 0 0 0.5] WeaponSystem
  (Utilities|IsValid (Variables|Default|GetCurrentWeaponActor)
    (:Is%20Valid
      (Actor|DestroyActor (Variables|Default|GetCurrentWeaponActor)))
    (:Is%20Not%20Valid
      _))
  (bind _returnvalue (Game|SpawnActorfromClass (Utilities|Array|Get(acopy) (Variables|Default|GetWeaponList) (Variables|Default|GetWeaponIndex)) (Math|Transform|MakeTransform "0, 0, 0" "0, 0, 0" "0.000000,0.000000,0.000000") "AlwaysSpawn" "MultiplyWithRoot" 0 0))
  (bind _output_get (Variables|Default|SetCurrentWeaponActor _returnvalue))
  (Transformation|AttachComponentToComponent _output_get (Variables|Collision|GetCapsuleComponent) "" "SnapToTarget" "SnapToTarget" "SnapToTarget" true)
  (Transformation|SetActorRelativeTransform _output_get (Math|Transform|MakeTransform "20.000000,15.000000,60.000000" "0, 0, 0" "0.250000,0.250000,0.250000") false false))

(event Input|EnhancedActionEvents|EnhancedInputActionIA_Shoot
  (params (ActionValue :type Boolean) (ElapsedSeconds :type Float%20%28double-precision%29) (TriggeredSeconds :type Float%20%28double-precision%29) (InputAction :type Input%20Action%20Object%20Reference :default "/Game/_Game/Blueprints/Input/IA_Shoot.IA_Shoot"))
  ;[1 0 0 0.5] WeaponSystem
  (Class|BPIWeapon|Shoot(Message) (Variables|Default|GetCurrentWeaponActor))
  (CallFunction|WeaponUpdate))

(event Input|EnhancedActionEvents|EnhancedInputActionIA_Slash
  (params (ActionValue :type Boolean) (ElapsedSeconds :type Float%20%28double-precision%29) (TriggeredSeconds :type Float%20%28double-precision%29) (InputAction :type Input%20Action%20Object%20Reference :default "/Game/_Game/Blueprints/Input/IA_Slash.IA_Slash"))
  ;[1 0 0 0.5] WeaponSystem
  (:Triggered
    (Utilities|FlowControl|DoOnce false :!label _label
      (:Completed
        (Class|BPISlash|Slash(Message) (Variables|/Script/Engine.ChildActorComponent|GetChildActor (Variables|Default|GetBP_Knife))))))
  (:Completed
    (goto _label Reset)))

(event Input|EnhancedActionEvents|EnhancedInputActionIA_ChangeWeaponDown
  (params (ActionValue :type Boolean) (ElapsedSeconds :type Float%20%28double-precision%29) (TriggeredSeconds :type Float%20%28double-precision%29) (InputAction :type Input%20Action%20Object%20Reference :default "/Game/_Game/Blueprints/Input/IA_ChangeWeaponDown.IA_ChangeWeaponDown"))
  (bind _weaponlist (Variables|Default|GetWeaponList))
  (bind _returnvalue (Utilities|Array|Length _weaponlist))
  ;[1 0 0 0.5] WeaponSystem
  (if (> _returnvalue 1)
    (bind _result (Math|Integer|IncrementInt (Variables|Default|GetWeaponIndex) :!label _label)
      (:%20%20
        (Variables|Default|SetWeaponIndex (Math|Integer|%(Integer) _result _returnvalue))
        (if (<= (Utilities|Array|Get(acopy) (Variables|Default|GetAmmoList) (Variables|Default|GetWeaponIndex)) 0)
          (goto _label)
          (else
            (CallFunction|ChangeWeaponMesh)
            (CallFunction|WeaponUpdate)))))))

(event Input|EnhancedActionEvents|EnhancedInputActionIA_ChangeWeaponUp
  (params (ActionValue :type Boolean) (ElapsedSeconds :type Float%20%28double-precision%29) (TriggeredSeconds :type Float%20%28double-precision%29) (InputAction :type Input%20Action%20Object%20Reference :default "/Game/_Game/Blueprints/Input/IA_ChangeWeaponUp.IA_ChangeWeaponUp"))
  (bind _weaponlist (Variables|Default|GetWeaponList))
  (bind _returnvalue (Utilities|Array|Length _weaponlist))
  ;[1 0 0 0.5] WeaponSystem
  (if (> _returnvalue 1)
    (bind _result (Math|Integer|DecrementInt (Variables|Default|GetWeaponIndex) :!label _label)
      (:%20%20
        (if (< _result 0)
          (Variables|Default|SetWeaponIndex (+ _result _returnvalue))
          (else
            (Variables|Default|SetWeaponIndex _result)))
        (if (<= (Utilities|Array|Get(acopy) (Variables|Default|GetAmmoList) (Variables|Default|GetWeaponIndex)) 0)
          (goto _label)
          (else
            (CallFunction|ChangeWeaponMesh)
            (CallFunction|WeaponUpdate)))))))

(fn ConstructionScript)

(fn GetRandomColor
  (params (Array :type Array%20of%20Material%20Interface%20Object%20References))
  (return (Utilities|Array|Get(acopy) Array (Math|Random|RandomInteger (Utilities|Array|Length Array)))))

(fn HealthUpdate
  (Variables|/Game/_Game/Blueprints/UI/HUD/WBP_HealthBar.WBP_HealthBar_C|SetHealthLeft (Variables|/Game/_Game/Blueprints/UI/HUD/WBP_HUD.WBP_HUD_C|GetWBP_HealthBar (Variables|Default|GetHUD)) (Variables|Default|GetHealth)))

(fn WeaponUpdate
  (bind _weaponindex (Variables|Default|GetWeaponIndex))
  (bind _hud (Variables|Default|GetHUD))
  (bind _wbp_weapon (Variables|/Game/_Game/Blueprints/UI/HUD/WBP_HUD.WBP_HUD_C|GetWBP_Weapon _hud))
  (Variables|/Game/_Game/Blueprints/UI/HUD/WBP_Weapon.WBP_Weapon_C|SetColorIndex _wbp_weapon _weaponindex)
  (Variables|/Game/_Game/Blueprints/UI/HUD/WBP_Weapon.WBP_Weapon_C|SetAmmoDisplayed _wbp_weapon (Utilities|Array|Get(acopy) (Variables|Default|GetAmmoList) _weaponindex)))
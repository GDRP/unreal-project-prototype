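; BP_FlameThrower is a firearm Blueprint that shoots short-range flame projectiles.
; Shoot spawns a BP_Flame at the Arrow component and moves it forward by Range over half a second.
; Each shot decrements the player BP_RattCharacter's ammo for the current weapon and calls NoAmmoLeft when empty.
; A DoOnce gate reset after a Rate delay caps the fire rate.
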(event EventShoot
  (bind _arrow (Variables|Default|GetArrow))
  (bind _arrow_2 (Variables|Default|GetArrow))
  (Utilities|FlowControl|DoOnce false :!label _label
    (:Completed
      (Utilities|FlowControl|Sequence
        (:then_0
          (bind _returnvalue (Game|SpawnActorfromClass "/Game/_Game/Blueprints/Weapons/Projectiles/BP_Flame.BP_Flame_C" (Math|Transform|MakeTransform (Transformation|GetWorldLocation _arrow_2) (Transformation|GetWorldRotation _arrow_2) "1.000000,1.000000,1.000000") "Undefined" "MultiplyWithRoot" 0 0))
          (Default|Moveto _returnvalue (+ (Transformation|GetWorldLocation _arrow) (* (Math|Vector|GetForwardVector _arrow) (Variables|Default|GetRange))) 0.5))
        (:then_1
          (bind _asbp_ratt_character (Utilities|Casting|CastToBP_RattCharacter (Game|GetPlayerCharacter 0)))
          (bind _result (Math|Integer|DecrementInt (Utilities|Array|Get(acopy) (Variables|/Game/_Game/Blueprints/Character/Player/BP_RattCharacter.BP_RattCharacter_C|GetAmmoList _asbp_ratt_character) (Variables|/Game/_Game/Blueprints/Character/Player/BP_RattCharacter.BP_RattCharacter_C|GetWeaponIndex _asbp_ratt_character)))
            (:%20%20
              (if (<= _result 0)
                (Default|NoAmmoLeft _asbp_ratt_character)))))
        (:then_2
          (Utilities|FlowControl|Delay (Variables|Default|GetRate))
          (goto _label Reset))))))

(fn ConstructionScript
  (|CallParentFunction))
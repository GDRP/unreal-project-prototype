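; BP_Pistol is a firearm Blueprint that fires projectiles when its Shoot event is called.
; Each shot spawns a BP_Bullet at the Arrow component's transform and calls its MoveTo toward a point Range units along the arrow's forward vector over one second.
; A DoOnce gate, reset after a Rate delay, limits the fire rate.
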(event EventShoot
  (bind _arrow (Variables|Default|GetArrow))
  (bind _arrow_2 (Variables|Default|GetArrow))
  (Utilities|FlowControl|DoOnce false :!label _label
    (:Completed
      (Utilities|FlowControl|Sequence
        (:then_0
          (bind _returnvalue (Game|SpawnActorfromClass "/Game/_Game/Blueprints/Weapons/Projectiles/BP_Bullet.BP_Bullet_C" (Math|Transform|MakeTransform (Transformation|GetWorldLocation _arrow_2) (Transformation|GetWorldRotation _arrow_2) "1.000000,1.000000,1.000000") "Undefined" "MultiplyWithRoot" 0 0))
          (Default|Moveto _returnvalue (+ (Transformation|GetWorldLocation _arrow) (* (Math|Vector|GetForwardVector _arrow) (Variables|Default|GetRange))) 1.0))
        (:then_1
          (Utilities|FlowControl|Delay (Variables|Default|GetRate))
          (goto _label Reset))))))

(fn ConstructionScript
  (|CallParentFunction))
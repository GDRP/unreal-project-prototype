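; Shotgun firearm Blueprint whose Shoot event fires a horizontal fan of BP_Bullet actors from its Arrow component.
; Each bullet's yaw is offset by SpreadAngle around the center, then MoveTo sends it forward to Range over one second.
; Each shot takes one round from player zero's BP_RattCharacter AmmoList and calls NoAmmoLeft when empty.
; A DoOnce gate, reset after a Rate delay, limits fire rate.
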(event EventShoot
  (bind _arrow (Variables|Default|GetArrow))
  (bind _bulletnumber (Variables|Default|GetBulletNumber))
  (bind _returnvalue (Transformation|GetWorldRotation _arrow))
  (bind _returnvalue_2 (- _bulletnumber 1))
  (Utilities|FlowControl|DoOnce false :!label _label
    (:Completed
      (Utilities|FlowControl|Sequence
        (:then_0
          (for _index (range 0 _returnvalue_2)
            (bind _returnvalue_3 (Game|SpawnActorfromClass "/Game/_Game/Blueprints/Weapons/Projectiles/BP_Bullet.BP_Bullet_C" (Math|Transform|MakeTransform (Transformation|GetWorldLocation _arrow) (Math|Rotator|MakeRotator (.roll _returnvalue) (.pitch _returnvalue) (+ (.yaw _returnvalue) (* (- _index (/ _returnvalue_2 2.0)) (Variables|Default|GetSpreadAngle)))) "1.000000,1.000000,1.000000") "Undefined" "MultiplyWithRoot" 0 0))
            (Default|Moveto _returnvalue_3 (+ (Transformation|GetWorldLocation (Variables|Default|GetArrow)) (* (Transformation|GetActorForwardVector _returnvalue_3) (Variables|Default|GetRange))) 1.0)))
        (:then_1
          (bind _asbp_ratt_character (Utilities|Casting|CastToBP_RattCharacter (Game|GetPlayerCharacter 0)))
          (bind _result (Math|Integer|DecrementInt (Utilities|Array|Get(acopy) (Variables|/Game/_Game/Blueprints/Character/Player/BP_RattCharacter.BP_RattCharacter_C|GetAmmoList _asbp_ratt_character) (Variables|/Game/_Game/Blueprints/Character/Player/BP_RattCharacter.BP_RattCharacter_C|GetWeaponIndex _asbp_ratt_character)))
            (:%20%20
              (if (<= _result 0)
                (Default|NoAmmoLeft _asbp_ratt_character)))))
        (:then_2
          (Utilities|FlowControl|Delay (Variables|Default|GetRate))
          (goto _label Reset))))))

(fn ConstructionScript
  (|CallParentFunction))
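; BP_SniperRifle is a firearm that fires a BP_SniperBullet along its arrow's forward direction.
; While ready to fire, Tick draws a debug line trace against pawns, apparently as a laser sight.
; Shoot moves the spawned bullet to max range, decrements the player character's ammo, signals when empty, and re-arms after a Rate delay via DoOnce.
; An unconnected sphere-trace branch that hurts orcs never runs.
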(event EventShoot
  (bind _arrow (Variables|Default|GetArrow))
  (bind _arrow_2 (Variables|Default|GetArrow))
  (Utilities|FlowControl|DoOnce false :!label _label
    (:Completed
      (Utilities|FlowControl|Sequence
        (:then_0
          (bind _returnvalue (Game|SpawnActorfromClass "/Game/_Game/Blueprints/Weapons/Projectiles/BP_SniperBullet.BP_SniperBullet_C" (Math|Transform|MakeTransform (Transformation|GetWorldLocation _arrow) (Transformation|GetWorldRotation _arrow) "1.000000,1.000000,1.000000") "Undefined" "MultiplyWithRoot" 0 0))
          (Default|Moveto _returnvalue (+ (Transformation|GetWorldLocation _arrow_2) (* (Math|Vector|GetForwardVector _arrow_2) (Variables|Default|GetRange))) 0.5)
          (Variables|Default|SetbCanShoot false))
        (:then_1
          (bind _asbp_ratt_character (Utilities|Casting|CastToBP_RattCharacter (Game|GetPlayerCharacter 0)))
          (bind _result (Math|Integer|DecrementInt (Utilities|Array|Get(acopy) (Variables|/Game/_Game/Blueprints/Character/Player/BP_RattCharacter.BP_RattCharacter_C|GetAmmoList _asbp_ratt_character) (Variables|/Game/_Game/Blueprints/Character/Player/BP_RattCharacter.BP_RattCharacter_C|GetWeaponIndex _asbp_ratt_character)))
            (:%20%20
              (if (<= _result 0)
                (Default|NoAmmoLeft _asbp_ratt_character)))))
        (:then_2
          (Utilities|FlowControl|Delay (Variables|Default|GetRate))
          (Variables|Default|SetbCanShoot true)
          (goto _label Reset))))))

(event EventTick
  (params (DeltaSeconds :type Float%20%28single-precision%29))
  (bind _arrow (Variables|Default|GetArrow))
  (bind _returnvalue (Transformation|GetWorldLocation _arrow))
  (if (Variables|Default|GetbCanShoot)
    (Class|KismetSystemLibrary|LineTraceMultiforObjects _returnvalue (+ _returnvalue (* (Math|Vector|GetForwardVector _arrow) (Variables|Default|GetRange))) (Utilities|Array|MakeArray "ObjectTypeQuery3") false 0 "ForDuration" true "(R=1.000000,G=0.000000,B=0.000000,A=1.000000)" "(R=1.000000,G=0.000000,B=0.000000,A=1.000000)" 0.02)))

(event EventBeginPlay
  (Variables|Default|SetbCanShoot true))

(fn ConstructionScript
  (|CallParentFunction))
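; BP_WeaponAmoPickUpBase is an ammo pickup actor, named as a base, that refills one weapon's ammo for the player character.
; On overlap with a BP_RattCharacter, it adds AmmoAmount to that character's AmmoList at WeaponIndex, calls WeaponUpdate, then destroys itself.
; BeginPlay hard-sets both the weapon index and amount, overwriting any values set on the defaults or placed instances.
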(event Collision|EventActorBeginOverlap
  (params (OtherActor :type Actor%20Object%20Reference))
  (bind _asbp_ratt_character (Utilities|Casting|CastToBP_RattCharacter OtherActor))
  (Utilities|Array|SetArrayElem (Variables|/Game/_Game/Blueprints/Character/Player/BP_RattCharacter.BP_RattCharacter_C|GetAmmoList _asbp_ratt_character) (Variables|Default|GetWeaponIndex) (+ (Utilities|Array|Get(acopy) (Variables|/Game/_Game/Blueprints/Character/Player/BP_RattCharacter.BP_RattCharacter_C|GetAmmoList _asbp_ratt_character) (Variables|Default|GetWeaponIndex)) (Variables|Default|GetAmmoAmount)))
  (Default|WeaponUpdate _asbp_ratt_character)
  (Actor|DestroyActor))

(event EventBeginPlay
  (Variables|Default|SetWeaponIndex 0)
  (Variables|Default|SetAmmoAmount 1))

(fn ConstructionScript)
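; BP_Knife is a melee weapon that damages orcs with a timed slash.
; Its Cube acts as the hitbox, hidden at zero scale until Slash offsets it by SlashLocation, then collapsed again after SlashDuration.
; Overlapping a BP_Orc calls Hurt and flags a hit.
; A slash that ends without a hit ends the combo on the player's BP_RattCharacter HUD widget.
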(event OnComponentBeginOverlap(Cube)
  (params (OverlappedComponent :type Primitive%20Component%20Object%20Reference) (OtherActor :type Actor%20Object%20Reference) (OtherComp :type Primitive%20Component%20Object%20Reference) (OtherBodyIndex :type Integer) (bFromSweep :type Boolean) (SweepResult :type Hit%20Result%20Structure%20%28by%20ref%29))
  (bind _asbp_orc (Utilities|Casting|CastToBP_Orc OtherActor))
  (Default|Hurt _asbp_orc)
  (Variables|Default|SetbHasHit true))

(event EventSlash
  (bind _cube (Variables|Default|GetCube))
  (Transformation|SetRelativeTransform _cube (Math|Transform|MakeTransform (+ (Variables|/Script/Engine.SceneComponent|GetRelativeLocation _cube) (Variables|Default|GetSlashLocation)) "0, 0, 0" "1.000000,1.000000,1.000000") false false)
  (Utilities|FlowControl|Delay (Variables|Default|GetSlashDuration))
  (Transformation|SetRelativeTransform _cube (Math|Transform|MakeTransform "0, 0, 0" "0, 0, 0" "0.000000,0.000000,0.000000") false false)
  (if (Variables|Default|GetbHasHit)
    (Variables|Default|SetbHasHit false)
    (else
      (bind _asbp_ratt_character (Utilities|Casting|CastToBP_RattCharacter (Game|GetPlayerCharacter 0)))
      (Default|EndCombo (Variables|/Game/_Game/Blueprints/UI/HUD/WBP_HUD.WBP_HUD_C|GetWBP_Combo (Variables|/Game/_Game/Blueprints/Character/Player/BP_RattCharacter.BP_RattCharacter_C|GetHUD _asbp_ratt_character))))))

(event EventBeginPlay
  (Transformation|SetRelativeTransform (Variables|Default|GetCube) (Math|Transform|MakeTransform "0, 0, 0" "0, 0, 0" "0.000000,0.000000,0.000000") false false))

(fn ConstructionScript)
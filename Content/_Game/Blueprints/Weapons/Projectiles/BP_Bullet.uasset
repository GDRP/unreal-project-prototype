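; BP_Bullet is a projectile that hurts orcs and ends the player's combo if it reaches its destination.
; MoveTo slides the root component to a destination over a given time, then calls EndCombo on the BP_RattCharacter HUD's combo widget and destroys the bullet.
; Sphere overlaps with BP_Orc call Hurt and destroy it early, while BP_Lock overlaps only destroy it.
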(event OnComponentBeginOverlap(Sphere)
  (params (OverlappedComponent :type Primitive%20Component%20Object%20Reference) (OtherActor :type Actor%20Object%20Reference) (OtherComp :type Primitive%20Component%20Object%20Reference) (OtherBodyIndex :type Integer) (bFromSweep :type Boolean) (SweepResult :type Hit%20Result%20Structure%20%28by%20ref%29))
  (bind _asbp_orc (Utilities|Casting|CastToBP_Orc OtherActor)
    (:then
      (Default|Hurt _asbp_orc))
    (:CastFailed
      (Utilities|Casting|CastToBP_Lock OtherActor)))
  (Actor|DestroyActor))

(event Custom|Move%20To
  (params (Destination :type Vector) (Time :type Float%20%28double-precision%29))
  (Components|MoveComponentTo (Variables|Default|GetDefaultSceneRoot) Destination (Transformation|GetWorldRotation (Variables|Default|GetSphere)) false false Time false)
  (bind _asbp_ratt_character (Utilities|Casting|CastToBP_RattCharacter (Game|GetPlayerCharacter 0)))
  (Default|EndCombo (Variables|/Game/_Game/Blueprints/UI/HUD/WBP_HUD.WBP_HUD_C|GetWBP_Combo (Variables|/Game/_Game/Blueprints/Character/Player/BP_RattCharacter.BP_RattCharacter_C|GetHUD _asbp_ratt_character)))
  (Actor|DestroyActor))

(fn ConstructionScript)
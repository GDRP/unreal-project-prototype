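; BP_Explosion is a short-lived explosion actor, filed under weapon projectiles, that shows an expanding sphere.
; Each tick it scales the Sphere component toward its current scale times ScaleMultiplier, using constant-rate interpolation capped by GrowthSpeed.
; Because the target is recomputed from the current scale, the scaling continues until the actor destroys itself after Duration.
; The graph itself applies no damage and handles no collisions.
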(event EventBeginPlay
  (Utilities|FlowControl|Delay (Variables|Default|GetDuration))
  (Actor|DestroyActor))

(event EventTick
  (params (DeltaSeconds :type Float%20%28single-precision%29))
  (bind _sphere (Variables|Default|GetSphere))
  (bind _returnvalue (Transformation|GetWorldScale _sphere))
  (Transformation|SetWorldScale3D _sphere (Math|Interpolation|VInterptoConstant _returnvalue (* _returnvalue (Variables|Default|GetScaleMultiplier)) DeltaSeconds (Variables|Default|GetGrowthSpeed))))

(fn ConstructionScript)
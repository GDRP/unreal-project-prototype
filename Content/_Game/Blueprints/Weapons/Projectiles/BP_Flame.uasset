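; Flame projectile that hurts orcs and breaks the player's combo on a miss.
; MoveTo glides the root to a slightly lowered destination, then after a short delay destroys the actor, calling EndCombo on the HUD if nothing was hit.
; Sphere overlap with an orc hurts it, halts movement and decrements PhysicalDuration, destroying the flame when depleted.
; Overlapping a BP_Lock only halts movement.
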(event OnComponentBeginOverlap(Sphere)
  (params (OverlappedComponent :type Primitive%20Component%20Object%20Reference) (OtherActor :type Actor%20Object%20Reference) (OtherComp :type Primitive%20Component%20Object%20Reference) (OtherBodyIndex :type Integer) (bFromSweep :type Boolean) (SweepResult :type Hit%20Result%20Structure%20%28by%20ref%29))
  (bind _asbp_orc (Utilities|Casting|CastToBP_Orc OtherActor)
    (:then
      (Default|Hurt _asbp_orc)
      (Variables|Default|SetbHasHit true)
      (Utilities|FlowControl|Sequence
        (:then_0
          (Components|MoveComponentTo (Variables|Default|GetDefaultSceneRoot) (Math|Vector|MakeVector (.X (Math|Vector|BreakVector (stale Custom|Move%20To Destination))) (.Y (Math|Vector|BreakVector (stale Custom|Move%20To Destination))) (- (.Z (Math|Vector|BreakVector (stale Custom|Move%20To Destination))) 5e+01)) (Transformation|GetWorldRotation (Variables|Default|GetSphere)) false false (stale Custom|Move%20To Time) false) ; enters at Stop
        )
        (:then_1
          (bind _result (Math|Integer|DecrementInt (Variables|Default|GetPhysicalDuration))
            (:%20%20
              (if (<= _result 0)
                (Actor|DestroyActor)))))))
    (:CastFailed
      (Utilities|Casting|CastToBP_Lock OtherActor)
      (Components|MoveComponentTo (Variables|Default|GetDefaultSceneRoot) (Math|Vector|MakeVector (.X (Math|Vector|BreakVector (stale Custom|Move%20To Destination))) (.Y (Math|Vector|BreakVector (stale Custom|Move%20To Destination))) (- (.Z (Math|Vector|BreakVector (stale Custom|Move%20To Destination))) 5e+01)) (Transformation|GetWorldRotation (Variables|Default|GetSphere)) false false (stale Custom|Move%20To Time) false) ; enters at Stop
    )))

(event Custom|Move%20To
  (params (Destination :type Vector) (Time :type Float%20%28double-precision%29))
  (bind (_x _y _z) (Math|Vector|BreakVector Destination))
  (Components|MoveComponentTo (Variables|Default|GetDefaultSceneRoot) (Math|Vector|MakeVector _x _y (- _z 5e+01)) (Transformation|GetWorldRotation (Variables|Default|GetSphere)) false false Time false)
  (Utilities|FlowControl|Delay 2.0)
  (if (Variables|Default|GetbHasHit)
    _
    (else
      (bind _asbp_ratt_character (Utilities|Casting|CastToBP_RattCharacter (Game|GetPlayerCharacter 0)))
      (Default|EndCombo (Variables|/Game/_Game/Blueprints/UI/HUD/WBP_HUD.WBP_HUD_C|GetWBP_Combo (Variables|/Game/_Game/Blueprints/Character/Player/BP_RattCharacter.BP_RattCharacter_C|GetHUD _asbp_ratt_character)))))
  (Actor|DestroyActor))

(fn ConstructionScript)
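; Rocket projectile that glides to a given destination and blows up on arrival, or earlier on overlapping an orc or lock.
; BlowUp spawns an explosion and runs three concentric sphere traces of growing radius, hurting orcs on each pass, so closer ones take repeated hits.
; It then destroys itself, first ending the player's HUD combo if nothing was hit.
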(event OnComponentBeginOverlap(Head)
  (params (OverlappedComponent :type Primitive%20Component%20Object%20Reference) (OtherActor :type Actor%20Object%20Reference) (OtherComp :type Primitive%20Component%20Object%20Reference) (OtherBodyIndex :type Integer) (bFromSweep :type Boolean) (SweepResult :type Hit%20Result%20Structure%20%28by%20ref%29))
  (Utilities|Casting|CastToBP_Orc OtherActor
    (:then
      _)
    (:CastFailed
      (Utilities|Casting|CastToBP_Lock OtherActor)))
  (CallFunction|BlowUp))

(event Custom|Move%20To
  (params (Destination :type Vector) (Time :type Float%20%28double-precision%29))
  (Components|MoveComponentTo (Variables|Default|GetDefaultSceneRoot) Destination (Transformation|GetWorldRotation (Variables|Default|GetHead)) false false Time false)
  (CallFunction|BlowUp))

(fn ConstructionScript)

(fn BlowUp
  (bind _head (Variables|Default|GetHead))
  (bind _returnvalue (Transformation|GetWorldLocation _head))
  (Game|SpawnActorfromClass "/Game/_Game/Blueprints/Weapons/Projectiles/BP_Explosion.BP_Explosion_C" (Math|Transform|MakeTransform (Transformation|GetWorldLocation (Variables|Default|GetHead)) "0, 0, 0" "1.000000,1.000000,1.000000") "Undefined" "MultiplyWithRoot" 0 0)
  (for _index (range 0 2)
    (bind (_outhits _returnvalue_2) (Collision|MultiSphereTraceForObjects _returnvalue _returnvalue (* (Variables|Default|GetRadius) (+ _index 1)) (Utilities|Array|MakeArray "ObjectTypeQuery3") false 0 "None" true "(R=1.000000,G=0.000000,B=0.000000,A=1.000000)" "(R=0.000000,G=1.000000,B=0.000000,A=1.000000)" 1.0))
    (for _array_element _outhits
      (bind _asbp_orc (Utilities|Casting|CastToBP_Orc (.HitActor (Collision|BreakHitResult _array_element))))
      (Default|Hurt _asbp_orc)
      (if _returnvalue_2
        (Variables|Default|SetbHasHit true))))
  (if (Variables|Default|GetbHasHit)
    _
    (else
      (bind _asbp_ratt_character (Utilities|Casting|CastToBP_RattCharacter (Game|GetPlayerCharacter 0)))
      (Default|EndCombo (Variables|/Game/_Game/Blueprints/UI/HUD/WBP_HUD.WBP_HUD_C|GetWBP_Combo (Variables|/Game/_Game/Blueprints/Character/Player/BP_RattCharacter.BP_RattCharacter_C|GetHUD _asbp_ratt_character)))))
  (Actor|DestroyActor))